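; Stalactite hazard actor that destroys any Player-tagged actor overlapping its box and moves with the player's gravity state.
; Each tick it polls GravityLow on the ThirdPersonCharacter1 player, using a boolean latch so the timeline triggers only on state changes.
; Low gravity plays the timeline, lerping the actor upward from its BeginPlay position with a swept move, and normal gravity reverses it.
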(event `self.Box.OnComponentBeginOverlap`
  (params (OverlappedComponent :type "PrimitiveComponent Object Reference") (OtherActor :type "Actor Object Reference") (OtherComp :type "PrimitiveComponent Object Reference") (OtherBodyIndex :type Integer) (bFromSweep :type Boolean) (SweepResult :type "HitResult Structure (by ref)"))
  (if (`self.ActorHasTag` OtherActor "Player")
    (`self.K2_DestroyActor` OtherActor)))

(event `self.ReceiveBeginPlay`
  (set `self.InitialPos` (`self.K2_GetActorLocation`)))

(event `self.ReceiveTick`
  (params (DeltaSeconds :type "Float (single-precision)"))
  (bind (_initialpos_x _initialpos_y _initialpos_z) (`KismetMathLibrary.BreakVector` (`self.InitialPos`)))
  (bind _asthird_person_character_1 (cast `/Game/Matéo/Character/ThirdPersonCharacter1` (`GameplayStatics.GetPlayerCharacter` 0)))
  (if (`/Game/Matéo/Character/ThirdPersonCharacter1.GravityLow` _asthird_person_character_1)
    (if (`self.istrig1`)
      (set `self.istrig1` false)
      (bind (_direction _newtrack_0) (`Timeline|Timeline_0` :`NewTime` 1.0 :!label _label)
        (:`Update`
          (`self.K2_SetActorRelativeLocation` (`KismetMathLibrary.VLerp` (`self.InitialPos`) (`KismetMathLibrary.MakeVector` _initialpos_x _initialpos_y (+ _initialpos_z 250.0)) _newtrack_0) true))))
    (elif (not (`self.istrig1`))
      (set `self.istrig1` true)
      (goto _label :!via `Reverse`))))

(fn `UserConstructionScript`)
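; Breakable ground actor that shatters when its Box is overlapped while the player character meets a state and height condition.
; The Geometry Collection starts inactive and hidden behind an intact cube.
; On any overlap, it checks the player's PreviousCharastate and CharacterHigh, without testing which actor overlapped.
; If both pass, it destroys the cube, reveals and activates the fracture pieces, then removes itself after a short delay.
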(event `self.ReceiveBeginPlay`
  (`ActorComponent.SetActive` (`self.Cube6_GeometryCollection`) false false)
  (`SceneComponent.SetVisibility` (`self.Cube6_GeometryCollection`) false false))

(event `self.Box.OnComponentBeginOverlap`
  (params (OverlappedComponent :type "PrimitiveComponent Object Reference") (OtherActor :type "Actor Object Reference") (OtherComp :type "PrimitiveComponent Object Reference") (OtherBodyIndex :type Integer) (bFromSweep :type Boolean) (SweepResult :type "HitResult Structure (by ref)"))
  (bind _asthird_person_character_1 (cast `/Game/Matéo/Character/ThirdPersonCharacter1` (`GameplayStatics.GetPlayerCharacter` 0)))
  (if (and (== (`/Game/Matéo/Character/ThirdPersonCharacter1.previousCharastate` _asthird_person_character_1) 0) (`/Game/Matéo/Character/ThirdPersonCharacter1.CharacterHigh` _asthird_person_character_1))
    (`ActorComponent.K2_DestroyComponent` (`self.Cube`))
    (`ActorComponent.SetActive` (`self.Cube6_GeometryCollection`) true false)
    (`SceneComponent.SetVisibility` (`self.Cube6_GeometryCollection`) true false)
    (`KismetSystemLibrary.Delay` 1.0)
    (`self.K2_DestroyActor`)))

(fn `UserConstructionScript`)
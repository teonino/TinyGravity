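; Static stalactite hazard actor that destroys any actor tagged Player that overlaps its Box.
; BeginPlay stores the start location, and Tick polls the player character's GravityLow flag, setting Istrig1 to its inverse, though nothing here acts on that flag.
; A Timeline meant to lerp the location from the start point is never triggered and has a zero Z offset, so the graph never moves the stalactite.
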(event `self.Box.OnComponentBeginOverlap`
  (params (OverlappedComponent :type "PrimitiveComponent Object Reference") (OtherActor :type "Actor Object Reference") (OtherComp :type "PrimitiveComponent Object Reference") (OtherBodyIndex :type Integer) (bFromSweep :type Boolean) (SweepResult :type "HitResult Structure (by ref)"))
  (if (`self.ActorHasTag` OtherActor "Player")
    (`self.K2_DestroyActor` OtherActor)))

(event `self.ReceiveBeginPlay`
  (set `self.InitialPos` (`self.K2_GetActorLocation`)))

(event `self.ReceiveTick`
  (params (DeltaSeconds :type "Float (single-precision)"))
  (bind _asthird_person_character_1 (cast `/Game/Matéo/Character/ThirdPersonCharacter1` (`GameplayStatics.GetPlayerCharacter` 0)))
  (if (`/Game/Matéo/Character/ThirdPersonCharacter1.GravityLow` _asthird_person_character_1)
    (if (`self.istrig1`)
      (set `self.istrig1` false))
    (elif (not (`self.istrig1`))
      (set `self.istrig1` true))))

(fn `UserConstructionScript`)
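; Lantern Blueprint that rotates its Empty component when the player's low-gravity state changes.
; Tick polls GravityLow on the player's ThirdPersonCharacter1, with the Istrig1 flag ensuring each change triggers the timeline only once.
; The timeline plays when low gravity starts and reverses when it ends, driving a swept rotation lerp between neutral and a tilted angle.
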(event `self.ReceiveTick`
  (params (DeltaSeconds :type "Float (single-precision)"))
  (bind _asthird_person_character_1 (cast `/Game/Matéo/Character/ThirdPersonCharacter1` (`GameplayStatics.GetPlayerCharacter` 0)))
  (if (`/Game/Matéo/Character/ThirdPersonCharacter1.GravityLow` _asthird_person_character_1)
    (if (`self.Istrig 1`)
      (set `self.Istrig 1` false)
      (bind (_direction _newtrack_0) (`Timeline|Timeline_0` :`NewTime` 1.0 :!label _label)
        (:`Update`
          (`SceneComponent.K2_SetRelativeRotation` (`self.empty`) (`KismetMathLibrary.RLerp` (struct) (struct :`Pitch` 70.0) _newtrack_0) true false))))
    (elif (not (`self.Istrig 1`))
      (set `self.Istrig 1` true)
      (goto _label :!via `Reverse`))))

(fn `UserConstructionScript`)